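; BP_TensorFlowWeaponGenerator bridges the game to a TensorFlow component that generates new weapons from dismantled weapon data.
; It flags itself ready to use when training completes, then encodes incoming dismantled weapon structs as JSON and sends them to the component.
; Returned results are parsed from JSON into a weapon API struct and passed to ReceiveNewWeaponFromGenerator.
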(event `self.TensorflowComponent.OnTrainingComplete`
  (params (SummaryJson :type String))
  (`self.setReadyToUse` true))

(event `self.sendDismantledWeaponToGenerator`
  (params (JsonData :type "WeaponGeneratorAPIJsonData Structure (by ref)"))
  (`/TensorFlow/TensorflowComponent.SendJsonInput` (`self.TensorflowComponent`) (`SIOJsonObject.EncodeJson` (`SIOJLibrary.StructToJsonObject` JsonData))))

(event `self.TensorflowComponent.OnInputResults`
  (params (Results :type String))
  (bind _output_get (set `self.WeaponGeneratorAPIJsonDataStruct` (make `WeaponGeneratorAPIJsonData` "")))
  (`SIOJLibrary.JsonObjectToStruct` (`SIOJLibrary.Conv_JsonValueToJsonObject` (`SIOJsonValue.ValueFromJsonString` Results)) _output_get)
  (`self.receiveNewWeaponFromGenerator` (`self.WeaponGeneratorAPIJsonDataStruct`)))

(fn `UserConstructionScript`)
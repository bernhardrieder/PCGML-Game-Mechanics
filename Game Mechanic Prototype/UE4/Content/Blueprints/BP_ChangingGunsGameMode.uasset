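; Game mode for a mode called Changing Guns that spawns AI bots on demand through its SpawnNewBot event.
; The event runs an EQS spawn-location query that picks randomly from the best 25% of points.
; On success, each returned location gets a weighted random bot: rarely a hard advanced AI, otherwise an easy one or a tracker bot.
; Spawns adjust for collision and are skipped if still blocked.
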(event `self.spawnNewBot`
  (bind _returnvalue (`EnvQueryManager.RunEQSQuery` "/Game/Blueprints/EQS/BotSpawn/EQS_FindSpawnLocation.EQS_FindSpawnLocation" self "RandomBest25Pct"))
  (add `EnvQueryInstanceBlueprintWrapper.OnQueryFinishedEvent` _returnvalue (delegate `OnQueryFinishedEvent_Event_0`)))

(event `OnQueryFinishedEvent_Event_0`
  (params (QueryInstance :type "EnvQueryInstanceBlueprintWrapper Object Reference") (QueryStatus :type "EEnvQueryStatus Enum" :default "Processing"))
  (switch `EEnvQueryStatus` QueryStatus
    (:`Success`
      (for _array_element (`EnvQueryInstanceBlueprintWrapper.GetResultsAsLocations` QueryInstance)
        (`|SpawnActorFromClass` (select `bool` (<= (`KismetMathLibrary.RandomFloatInRange` 0.0 100.0) 10.0) :`false` (select `bool` (<= (`KismetMathLibrary.RandomFloatInRange` 0.0 100.0) 50.0) :`false` "/Game/Blueprints/AI/BP_TrackerBot.BP_TrackerBot_C" :`true` "/Game/Blueprints/AI/AdvancedAIBot/BP_AdvancedAI_Easy.BP_AdvancedAI_Easy_C" :!type "Actor Class Reference") :`true` "/Game/Blueprints/AI/AdvancedAIBot/BP_AdvancedAI_Hard.BP_AdvancedAI_Hard_C") (`KismetMathLibrary.MakeTransform` _array_element) "AdjustIfPossibleButDontSpawnIfColliding" "OverrideRootScale" null null)))))

(fn `UserConstructionScript`)
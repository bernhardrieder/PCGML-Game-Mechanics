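; Player pawn Blueprint that manages the local player's crosshair and HUD widgets.
; On BeginPlay, a locally controlled pawn creates both widgets and binds to its health component's change event, which hides them when health reaches zero.
; Tick enlarges the crosshair while the pawn is moving and restores it otherwise, without checking local control or widget validity.
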(event `self.ReceiveTick`
  (params (DeltaSeconds :type "Float (single-precision)"))
  (bind _crosshair (`self.Crosshair`))
  (if (`self.IsMoving`)
    (`/Game/UI/WBP_CrossHair.ScaleCrosshair` _crosshair 2.0)
    (else
      (`/Game/UI/WBP_CrossHair.ScaleCrosshair` _crosshair 1.0))))

(event `self.ReceiveBeginPlay`
  (if (`self.IsLocallyControlled`)
    (`|ExecutionSequence`
      (:`then_0`
        (bind _returnvalue (`|CreateWidget` "/Game/UI/WBP_CrossHair.WBP_CrossHair_C"))
        (`UserWidget.AddToViewport` _returnvalue 0)
        (set `self.Crosshair` _returnvalue))
      (:`then_1`
        (bind _returnvalue_2 (`|CreateWidget` "/Game/UI/InGame/WBP_HUD.WBP_HUD_C"))
        (`UserWidget.AddToViewport` _returnvalue_2 0)
        (set `self.HUD` _returnvalue_2))
      (:`then_2`
        (add `HealthComponent.OnHealthChangedEvent` (`self.HealthComp`) (delegate `OnHealthChangedEvent_Event_0`))))))

(event `OnHealthChangedEvent_Event_0`
  (params (OwningHealthComp :type "HealthComponent Object Reference") (Health :type "Float (double-precision)") (HealthDelta :type "Float (double-precision)") (CausedDamageType :type "DamageType Object Reference") (InstigatedBy :type "Controller Object Reference") (DamageCauser :type "Actor Object Reference"))
  (if (<= Health 0.0)
    (`Widget.SetVisibility` (`self.Crosshair`) "Hidden")
    (`Widget.SetVisibility` (`self.HUD`) "Hidden")))

(fn `UserConstructionScript`)
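; Bridge actor that uses a TensorFlow component to generate new weapons from dismantled weapon data.
; Training completion prints a message and flags the generator as ready to use.
; Incoming dismantled-weapon structs are encoded as JSON and sent to the component as input.
; Returned results are parsed from JSON into a weapon API struct and passed to ReceiveNewWeaponFromGenerator.
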(event `self.TensorflowComponent.OnTrainingComplete`
  (params (SummaryJson :type String))
  (`KismetSystemLibrary.PrintString` "Training Complete")
  (`self.setReadyToUse` true))

(event `self.sendDismantledWeaponToGenerator`
  (params (jsonData :type "WeaponGeneratorAPIJsonData Structure (by ref)"))
  (`/TensorFlow/TensorflowComponent.SendJsonInput` (`self.TensorflowComponent`) (`SIOJsonObject.EncodeJson` (`SIOJLibrary.StructToJsonObject` jsonData))))

(event `self.TensorflowComponent.OnInputResults`
  (params (Results :type String))
  (bind _output_get (set `self.WeaponGeneratorAPIJsonDataStruct` (make `WeaponGeneratorAPIJsonData` "")))
  (`SIOJLibrary.JsonObjectToStruct` (`SIOJLibrary.Conv_JsonValueToJsonObject` (`SIOJsonValue.ValueFromJsonString` Results)) _output_get)
  (`self.receiveNewWeaponFromGenerator` (`self.WeaponGeneratorAPIJsonDataStruct`)))

(fn `UserConstructionScript`)
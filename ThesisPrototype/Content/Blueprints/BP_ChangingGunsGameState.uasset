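; Game state Blueprint for ChangingGuns that reacts to wave state changes and handles the game over screen.
; On each WaveStateChanged event it prints the new state to screen.
; On Game Over it creates the WBP_GameOverMenu widget if none exists yet, adds it to the viewport, and switches the first player controller to UI-only input with a visible cursor.
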(event `self.waveStateChanged`
  (params (newState :type "EWaveState Enum" :default "WaitingToStart") (oldState :type "EWaveState Enum" :default "WaitingToStart"))
  (bind _returnvalue (`GameplayStatics.GetPlayerController` 0))
  (`KismetSystemLibrary.PrintString` (`|GetEnumeratorNameAsString` newState) true true (struct :`G` 0.66 :`B` 1.0 :`A` 1.0) 5.0)
  (switch `EWaveState` newState
    (:`GameOver`
      (`/Engine/EditorBlueprintResources/StandardMacros.IsValid` (`self.GameOverUi`)
        (:`Is Not Valid`
          (bind _returnvalue_2 (`|CreateWidget` "/Game/UI/WBP_GameOverMenu.WBP_GameOverMenu_C" _returnvalue))
          (bind _output_get (set `self.GameOverUi` _returnvalue_2))
          (`UserWidget.AddToViewport` _output_get 0)
          (`WidgetBlueprintLibrary.SetInputMode_UIOnlyEx` _returnvalue _returnvalue_2)
          (set `PlayerController.bShowMouseCursor` true _returnvalue))))))

(fn `UserConstructionScript`)
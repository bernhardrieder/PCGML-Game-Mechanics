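; Base AI bot Blueprint that runs a behavior tree and shows a world-space health bar above the pawn.
; On BeginPlay, with a valid AI controller, it starts the tree, initializes the bar from HealthComp's default health and binds to health changes.
; Health changes update the bar and hide it at zero health.
; While visible, the widget rotates toward the first player's camera every Tick.
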(event `self.ReceiveBeginPlay`
  (bind _returnvalue (`AIBlueprintHelperLibrary.GetAIController` self))
  (`/Engine/EditorBlueprintResources/StandardMacros.IsValid` _returnvalue
    (:`Is Valid`
      (`AIController.RunBehaviorTree` _returnvalue (`self.BehaviorTree`))
      (bind _aswbp_pawn_health_bar (cast `/Game/UI/InGame/WBP_PawnHealthBar` (`WidgetComponent.GetUserWidgetObject` (`self.HealthBarWidget`))))
      (bind _output_get (set `self.HealthBar` (`/Game/UI/InGame/WBP_PawnHealthBar.WBP_HealthBar` _aswbp_pawn_health_bar)))
      (bind _output_get_2 (set `/Game/UI/WBP_HealthBar.maxHealth` (`HealthComponent.DefaultHealth` (`self.HealthComp`)) _output_get))
      (`/Game/UI/WBP_HealthBar.UpdateHealth` _output_get _output_get_2)
      (add `HealthComponent.OnHealthChangedEvent` (`self.HealthComp`) (delegate `OnHealthChangedEvent_Event_0`)))))

(event `OnHealthChangedEvent_Event_0`
  (params (OwningHealthComp :type "HealthComponent Object Reference") (Health :type "Float (double-precision)") (HealthDelta :type "Float (double-precision)") (CausedDamageType :type "DamageType Object Reference") (InstigatedBy :type "Controller Object Reference") (DamageCauser :type "Actor Object Reference"))
  (`/Game/UI/WBP_HealthBar.UpdateHealth` (`self.HealthBar`) Health)
  (if (<= Health 0.0)
    (`SceneComponent.SetVisibility` (`self.HealthBarWidget`) false true)))

(event `self.ReceiveTick`
  (params (DeltaSeconds :type "Float (single-precision)"))
  (if (`SceneComponent.IsVisible` (`self.HealthBarWidget`))
    (`self.RotateHealthBarToPlayer`)))

(fn `RotateHealthBarToPlayer`
  (`SceneComponent.K2_SetWorldRotation` (`self.HealthBarWidget`) (`KismetMathLibrary.FindLookAtRotation` (`SceneComponent.K2_GetComponentLocation` (`self.HealthBarWidget`)) (`PlayerCameraManager.GetCameraLocation` (`GameplayStatics.GetPlayerCameraManager` 0))) false false))

(fn `UserConstructionScript`)
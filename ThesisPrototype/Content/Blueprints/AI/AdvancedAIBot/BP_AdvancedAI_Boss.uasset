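; Advanced AI boss character that stays dormant until the boss fight starts, then ends the game with a win screen when killed.
; A player hit switches the GameState to BossFight and fully restores the player's health, armor and extra lives.
; Tick polls that state to start the behavior tree and damage handling once, and turns the health bar toward the camera.
; Death disables player input and removes non-player ShooterCharacters.
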(event `OnHealthChangedEvent_Event_0`
  (params (OwningHealthComp :type "HealthComponent Object Reference") (Health :type "Float (double-precision)") (HealthDelta :type "Float (double-precision)") (CausedDamageType :type "DamageType Object Reference") (InstigatedBy :type "Controller Object Reference") (DamageCauser :type "Actor Object Reference"))
  (bind _returnvalue (`GameplayStatics.GetPlayerController` 0))
  (`/Game/UI/WBP_HealthBar.UpdateHealth` (`self.HealthBar`) Health)
  (if (<= Health 0.0)
    (`SceneComponent.SetVisibility` (`self.HealthBarWidget`) false true)
    (`self.DisableInput` _returnvalue _returnvalue)
    (bind _returnvalue_2 (`|CreateWidget` "/Game/UI/WBP_WinScreen.WBP_WinScreen_C" _returnvalue))
    (`UserWidget.AddToViewport` _returnvalue_2 0)
    (`WidgetBlueprintLibrary.SetInputMode_UIOnlyEx` _returnvalue _returnvalue_2)
    (set `PlayerController.bShowMouseCursor` true _returnvalue)
    (bind _asshooter_character (cast `ShooterCharacter` (`Controller.K2_GetPawn` _returnvalue)))
    (if (`self.IsPlayerControlled` _asshooter_character)
      (`self.StopFire` _asshooter_character)
      (bind _outactors (`GameplayStatics.GetAllActorsOfClass` "/Script/ThesisPrototype.ShooterCharacter"))
      (for _array_element _outactors
        (if (not (`self.IsPlayerControlled` _array_element))
          (`self.SetLifeSpan` _array_element 0.1))))))

(event `OnBossActivation`
  (bind _returnvalue (`AIBlueprintHelperLibrary.GetAIController` self))
  (if (not (`self.isActivated`))
    (set `self.isActivated` true)
    (`/Engine/EditorBlueprintResources/StandardMacros.IsValid` _returnvalue
      (:`Is Valid`
        (`AIController.RunBehaviorTree` _returnvalue "/Game/Blueprints/AI/AdvancedAIBot/BehaviorTrees/BT_AdvancedAI_Boss.BT_AdvancedAI_Boss")
        (`SceneComponent.SetVisibility` (`self.HealthBarWidget`) true true)
        (add `HealthComponent.OnHealthChangedEvent` (`self.HealthComp`) (delegate `OnHealthChangedEvent_Event_0`))
        (`HealthComponent.SetHandleDamageEnabled` (`self.HealthComp`) true)))))

(event `self.ReceiveBeginPlay`
  (bind _aschanging_guns_game_state (cast `ChangingGunsGameState` (`GameplayStatics.GetGameState`)))
  (set `self.GameState` _aschanging_guns_game_state)
  (add `HealthComponent.OnHealthChangedEvent` (`self.HealthComp`) (delegate `activate boss fight`))
  (bind _aswbp_pawn_health_bar (cast `/Game/UI/InGame/WBP_PawnHealthBar` (`WidgetComponent.GetUserWidgetObject` (`self.HealthBarWidget`))))
  (bind _output_get (set `self.HealthBar` (`/Game/UI/InGame/WBP_PawnHealthBar.WBP_HealthBar` _aswbp_pawn_health_bar)))
  (bind _output_get_2 (set `/Game/UI/WBP_HealthBar.maxHealth` (`HealthComponent.DefaultHealth` (`self.HealthComp`)) _output_get))
  (`/Game/UI/WBP_HealthBar.UpdateHealth` _output_get _output_get_2)
  (`SceneComponent.SetVisibility` (`self.HealthBarWidget`) false true))

(event `activate boss fight`
  (params (OwningHealthComp :type "HealthComponent Object Reference") (Health :type "Float (double-precision)") (HealthDelta :type "Float (double-precision)") (CausedDamageType :type "DamageType Object Reference") (InstigatedBy :type "Controller Object Reference") (DamageCauser :type "Actor Object Reference"))
  (if (`|EnumInequality` (`ChangingGunsGameState.WaveState` (`self.GameState`)) "BossFight")
    (bind _asshooter_character (cast `ShooterCharacter` DamageCauser))
    (if (`self.IsPlayerControlled` _asshooter_character)
      (`ChangingGunsGameState.SetWaveState` (`self.GameState`) "BossFight")
      (bind _healthcomp (`ShooterCharacter.HealthComp` _asshooter_character))
      (`HealthComponent.Heal` _healthcomp (`HealthComponent.DefaultHealth` _healthcomp))
      (`HealthComponent.RepairArmor` _healthcomp (`HealthComponent.DefaultArmor` _healthcomp))
      (`HealthComponent.RestoreExtraLife` _healthcomp (`HealthComponent.DefaultExtraLives` _healthcomp)))))

(event `self.ReceiveTick`
  (params (DeltaSeconds :type "Float (single-precision)"))
  (if (`|EnumEquality` (`ChangingGunsGameState.WaveState` (`self.GameState`)) "BossFight")
    (`self.OnBossActivation`)
    (if (`SceneComponent.IsVisible` (`self.HealthBarWidget`))
      (`self.RotateHealthBarToPlayer`))))

(fn `RotateHealthBarToPlayer`
  (`SceneComponent.K2_SetWorldRotation` (`self.HealthBarWidget`) (`KismetMathLibrary.FindLookAtRotation` (`SceneComponent.K2_GetComponentLocation` (`self.HealthBarWidget`)) (`PlayerCameraManager.GetCameraLocation` (`GameplayStatics.GetPlayerCameraManager` 0))) false false))

(fn `UserConstructionScript`)
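; Super speed power-up pickup that temporarily doubles the walking speed of the player who activates it.
; On activation it stores the player and multiplies their CharacterMovementComponent MaxWalkSpeed.
; On expiry it divides the speed back down if the player and component are still valid, then always calls the parent expiry logic.
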(event `self.OnActivated`
  (params (ActivatedFor :type "Actor Object Reference"))
  (bind _output_get (set `self.ActivatedForPlayer` ActivatedFor))
  (`/Engine/EditorBlueprintResources/StandardMacros.IsValid` _output_get
    (:`Is Valid`
      (bind _returnvalue (`self.GetComponentByClass` _output_get "/Script/Engine.CharacterMovementComponent"))
      (`/Engine/EditorBlueprintResources/StandardMacros.IsValid` _returnvalue
        (:`Is Valid`
          (set `CharacterMovementComponent.MaxWalkSpeed` (* (`CharacterMovementComponent.MaxWalkSpeed` _returnvalue) 2.0) _returnvalue))))))

(event `self.OnExpired`
  (bind _activatedforplayer (`self.ActivatedForPlayer`))
  (bind _returnvalue (`self.GetComponentByClass` _activatedforplayer "/Script/Engine.CharacterMovementComponent"))
  (`/Engine/EditorBlueprintResources/StandardMacros.IsValid` _activatedforplayer
    (:`Is Valid`
      (`/Engine/EditorBlueprintResources/StandardMacros.IsValid` _returnvalue
        (:`Is Valid`
          (set `CharacterMovementComponent.MaxWalkSpeed` (/ (`CharacterMovementComponent.MaxWalkSpeed` _returnvalue) 2.0) _returnvalue)
          (`parent.OnExpired`))
        (:`Is Not Valid`
          (`parent.OnExpired` :!label _label))))
    (:`Is Not Valid`
      (goto _label))))

(fn `UserConstructionScript`)